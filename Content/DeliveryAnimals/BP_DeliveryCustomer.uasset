(event `TryDeliver`
  (if (`self.Delivered`)
    _
    (elif (<= (`self.GetDistanceTo` (`GameplayStatics.GetPlayerPawn` 0)) 240.0)
      (bind _asbp_manhattan_game_mode (cast `/Game/ManhattanGameplay/BP_ManhattanGameMode` (`GameplayStatics.GetGameMode`)))
      (set `self.Delivered` true)
      (set `/Game/ManhattanGameplay/BP_ManhattanGameMode.DeliveriesCompleted` (+ (`/Game/ManhattanGameplay/BP_ManhattanGameMode.DeliveriesCompleted` _asbp_manhattan_game_mode) 1) _asbp_manhattan_game_mode)
      (`TextRenderComponent.K2_SetText` (`self.DeliveryPrompt`) (`KismetTextLibrary.Conv_StringToText` "Delivered - thank you!")))))

(event `self.ReceiveTick`
  (params (DeltaSeconds :type "Float (single-precision)"))
  (bind _deliveryprompt (`self.DeliveryPrompt`))
  (`|ExecutionSequence`
    (:`then_0`
      (`self.K2_SetActorRotation` (`KismetMathLibrary.MakeRotator` 0.0 0.0 (.yaw (`KismetMathLibrary.FindLookAtRotation` (`self.K2_GetActorLocation`) (`PlayerCameraManager.GetCameraLocation` (`GameplayStatics.GetPlayerCameraManager` 0))))))
      (if (`self.Delivered`)
        (`TextRenderComponent.K2_SetText` _deliveryprompt (`KismetTextLibrary.Conv_StringToText` "Delivered - thank you!"))
        (elif (<= (`self.GetDistanceTo` (`GameplayStatics.GetPlayerPawn` 0)) 240.0)
          (`TextRenderComponent.K2_SetText` _deliveryprompt (`KismetTextLibrary.Conv_StringToText` "[E] Deliver food"))
          (else
            (`TextRenderComponent.K2_SetText` _deliveryprompt (`KismetTextLibrary.Conv_StringToText` "Food delivery"))))))
    (:`then_1`
      (if (`PlayerController.WasInputKeyJustPressed` (`GameplayStatics.GetPlayerController` 0) "(")
        (`self.TryDeliver`)))))

(fn `UserConstructionScript`)