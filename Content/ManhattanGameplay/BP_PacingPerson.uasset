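; BP_PacingPerson is a pedestrian obstacle that paces back and forth and ends the run when the player pawn overlaps it.
; Each tick it sets its location to a sine offset along its forward vector around its spawn point, scaled by pace frequency and distance.
; A random phase chosen at BeginPlay desynchronizes multiple instances.
; On player overlap it calls EndRun on BP_ManhattanGameMode.
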(event `self.ReceiveBeginPlay`
  (set `self.PaceOrigin` (`self.K2_GetActorLocation`))
  (set `self.Phase` (`KismetMathLibrary.RandomFloatInRange` 0.0 6.283185)))

(event `self.ReceiveTick`
  (params (DeltaSeconds :type "Float (single-precision)"))
  (`self.K2_SetActorLocation` (+ (`self.PaceOrigin`) (* (`self.GetActorForwardVector`) (* (`KismetMathLibrary.Sin` (+ (* (`GameplayStatics.GetTimeSeconds`) (`self.PaceFrequency`)) (`self.Phase`))) (`self.PaceDistance`))))))

(event `self.ReceiveActorBeginOverlap`
  (params (OtherActor :type "Actor Object Reference"))
  (if (== OtherActor (`GameplayStatics.GetPlayerPawn` 0))
    (bind _asbp_manhattan_game_mode (cast `/Game/ManhattanGameplay/BP_ManhattanGameMode` (`GameplayStatics.GetGameMode`)))
    (`/Game/ManhattanGameplay/BP_ManhattanGameMode.EndRun` _asbp_manhattan_game_mode)))

(fn `UserConstructionScript`)